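; BP_Player is a player-controlled actor that moves freely along the world X, Y and Z axes.
; BeginPlay registers an Enhanced Input mapping context, and three axis input actions store their values on Triggered and Completed.
; Tick normalizes the combined input vector, scales it by Movespeed and delta time, and offsets the actor location directly without sweeping for collision.
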(event Input|EnhancedActionEvents|EnhancedInputActionInputAction_X
  (params (ActionValue :type Float%20%28double-precision%29) (ElapsedSeconds :type Float%20%28double-precision%29) (TriggeredSeconds :type Float%20%28double-precision%29) (InputAction :type Input%20Action%20Object%20Reference :default "/Game/BP/control/InputAction_X.InputAction_X"))
  ;[1 1 1] Input Action
  (:Triggered
    (Variables|Default|SetX ActionValue))
  (:Completed
    (Variables|Default|SetX ActionValue)))

(event Input|EnhancedActionEvents|EnhancedInputActionInputAction_Y
  (params (ActionValue :type Float%20%28double-precision%29) (ElapsedSeconds :type Float%20%28double-precision%29) (TriggeredSeconds :type Float%20%28double-precision%29) (InputAction :type Input%20Action%20Object%20Reference :default "/Game/BP/control/InputAction_Y.InputAction_Y"))
  ;[1 1 1] Input Action
  (:Triggered
    (Variables|Default|SetY ActionValue))
  (:Completed
    (Variables|Default|SetY ActionValue)))

(event Input|EnhancedActionEvents|EnhancedInputActionInputAction_Z
  (params (ActionValue :type Float%20%28double-precision%29) (ElapsedSeconds :type Float%20%28double-precision%29) (TriggeredSeconds :type Float%20%28double-precision%29) (InputAction :type Input%20Action%20Object%20Reference :default "/Game/BP/control/InputAction_Z.InputAction_Z"))
  ;[1 1 1] Input Action
  (:Triggered
    (Variables|Default|SetZ ActionValue))
  (:Completed
    (Variables|Default|SetZ ActionValue)))

(event EventBeginPlay
  ;[1 1 1] Mappting Context
  (Input|AddMappingContext (PlayerController|LocalPlayerSubsystems|GetEnhancedInputLocalPlayerSubsystem (Game|GetPlayerController 0)) "/Game/BP/control/InputMapping.InputMapping" 0 "(bIgnoreAllPressedKeysUntilRelease=True,bForceImmediately=False,bNotifyUserSettings=False)"))

(event Collision|EventActorBeginOverlap
  (params (OtherActor :type Actor%20Object%20Reference)))

(event EventTick
  (params (DeltaSeconds :type Float%20%28single-precision%29))
  ;[1 1 1] Input Location
  (Transformation|SetActorLocation (+ (Transformation|GetActorLocation) (* (* (Math|Vector|Normalize (Math|Vector|MakeVector (Variables|Default|GetX) (Variables|Default|GetY) (Variables|Default|GetZ))) (Variables|Default|Getmovespeed)) DeltaSeconds)) false false))

(fn ConstructionScript)